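; BP_PatrolRoutes defines an AI patrol route from the points of its PatrolRoutes spline.
; IncrementPatrolPoints steps CurrentIndex by Direction, reversing at the last point and at the first so the index ping-pongs along the spline instead of looping.
; GetPatrolPointsLocation returns the world-space location of the spline point at the current index.
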(event Custom|IncrementPatrolPoints
  (bind _output_get (Variables|Default|SetCurrentIndex (+ (Variables|Default|GetCurrentIndex) (Variables|Default|GetDirection))))
  (if (== _output_get (- (Spline|GetNumberOfSplinePoints (Variables|Default|GetPatrolRoutes)) 1))
    (Variables|Default|SetDirection -1)
    (elif (== (Variables|Default|GetCurrentIndex) 0)
      (Variables|Default|SetDirection 1))))

(fn ConstructionScript)

(fn GetPatrolPointsLocation
  (return (Spline|GetLocationatSplinePoint (Variables|Default|GetPatrolRoutes) (Variables|Default|GetCurrentIndex) "World")))